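; BP_Gauntlet_Character is a character Blueprint that sets up projectile object pooling.
; On BeginPlay it creates a pool of BP_ProjectileBase and adds the WBP_PoolerSTAT widget to the viewport.
; An unconnected chain, which never runs, would fetch a BP_PooledProjectile from the pool, place it just ahead of the character with a debug sphere, and activate it.
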(event EventBeginPlay
  (CallFunction|CreateObjectPool "/Game/_Game/Lesson12-09/BP_ProjectileBase.BP_ProjectileBase_C" (Variables|Default|GetInitial%20Size))
  (bind _returnvalue (UserInterface|CreateWidget "/Game/_Game/Lesson12-09/WBP_PoolerSTAT.WBP_PoolerSTAT_C"))
  (UserInterface|Viewport|AddtoViewport _returnvalue 0))

(event Input|KeyboardEvents|DebugKeyT
  (params (Key :type Key%20Structure :default "None") (ActionValue :type Input%20Action%20Value%20Structure)))

(fn ConstructionScript)