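; Player controller for the Gauntlet game that drives menus, pause, input mode and cursor visibility from the game state held in the GameInstance.
; BeginPlay adds the input mapping, creates the menu-stack widget, binds to state changes and picks main menu or play from the level name.
; Menu and pause states push a widget and pause; other states remove it and resume.
; Escape toggles pause, and cursor visibility also considers input device.
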(event `EnhancedInput|/Game/_Game/Input/Actions/Gameplay/IA_Escape`
  (params (ActionValue :type Boolean) (ElapsedSeconds :type "Float (double-precision)") (TriggeredSeconds :type "Float (double-precision)") (InputAction :type "InputAction Object Reference" :default "/Game/_Game/Input/Actions/Gameplay/IA_Escape.IA_Escape"))
  (bind _returnvalue (`Gauntlet_GameInstance.GetGameState` (`self.GameInstance`)))
  (:`Triggered`
    (if (`|EnumEquality` _returnvalue "InPlay")
      (`self.OnGameStateChange` "InPause")
      (elif (`|EnumEquality` _returnvalue "InPause")
        (`self.OnGameStateChange` "InPlay")))))

(event `self.ReceiveBeginPlay`
  (`|ExecutionSequence`
    (:`then_0`
      (`EnhancedInputSubsystemInterface.AddMappingContext` (subsystem `EnhancedInputLocalPlayerSubsystem`) "/Game/_Game/Input/IMC_TheGauntlet.IMC_TheGauntlet" 0 (struct)))
    (:`then_1`
      ; SetHUD and Menu
      (bind _returnvalue (`|CreateWidget` "/Game/_Game/UI/Widgets/WBP_MenuStacks.WBP_MenuStacks_C"))
      (bind _output_get (set `self.UIStacks` _returnvalue))
      (`UserWidget.AddToViewport` _output_get 0))
    (:`then_2`
      (bind _asgauntlet_game_instance (cast `Gauntlet_GameInstance` (`GameplayStatics.GetGameInstance`))
        (:`then`
          (bind _output_get_2 (set `self.GameInstance` _asgauntlet_game_instance))
          (`Gauntlet_GameInstance.SetGameState` _output_get_2 "InMainMenu")
          (add `Gauntlet_GameInstance.OnGameStateChanged` _output_get_2 (delegate `OnGameStateChange`)))
        (:`CastFailed`
          (`KismetSystemLibrary.PrintString` "ERROR - GameInstance" true true (struct :`R` 1.0 :`A` 1.0) 2.0 "E1"))))
    (:`then_3`
      (bind _returnvalue_2 (`GameplayStatics.GetCurrentLevelName` true))
      (`self.OnGameStateChange` (select `bool` (`KismetStringLibrary.EqualEqual_StrStr` _returnvalue_2 "Lvl_MainMenu") :`false` "InPlay" :`true` "InMainMenu" :!type "EGauntlet_GameState Enum")))))

(event `OnGameStateChange`
  (params (NewState :type "EGauntlet_GameState Enum" :default "InMainMenu"))
  (bind _uistacks (`self.UIStacks`))
  (`Gauntlet_GameInstance.SetGameState` (`self.GameInstance`) NewState)
  (switch `EGauntlet_GameState` NewState
    (:`InMainMenu`
      (`/Game/_Game/UI/Widgets/WBP_MenuStacks.PushMenu` (`self.UIStacks`) (select `EGauntlet_GameState` (`Gauntlet_GameInstance.GetGameState` (`self.GameInstance`)) :`InMainMenu` (`self.Menu Class`) :`InPause` (`self.Pause Class`)) :!label _label)
      (`WidgetBlueprintLibrary.SetInputMode_UIOnlyEx` self (`self.UIStacks`))
      (`self.ShowCursor`)
      (`GameplayStatics.SetGamePaused` true))
    (:`InPlay`
      (`WidgetBlueprintLibrary.SetInputMode_GameOnly` self :!label _label_2)
      (set `self.bShowMouseCursor` false)
      (`GameplayStatics.SetGamePaused` false)
      (`/Game/_Game/UI/Widgets/WBP_MenuStacks.RemoveMenu` _uistacks (`CommonActivatableWidgetContainerBase.GetActiveWidget` (`/Game/_Game/UI/Widgets/WBP_MenuStacks.MenuStack` _uistacks))))
    (:`InPause`
      (goto _label))
    (:`InLoading`
      (goto _label_2))
    (:`InSaving`
      (goto _label_2))))

(event `self.ReceiveDestroyed`
  (clear `Gauntlet_GameInstance.OnGameStateChanged` (`self.GameInstance`)))

(event `NewInputDevice`
  (params (IsMouseKeyboard :type Boolean))
  ; Detect Input Device
  (`Gauntlet_GameInstance.SetInputDevice` (`self.GameInstance`) (select `bool` IsMouseKeyboard :`false` "Gamepad" :`true` "MouseKeyboard" :!type "EGauntlet_InputDevice Enum"))
  (`self.ShowCursor`))

(event `ShowCursor`
  (bind _gameinstance (`self.GameInstance`))
  (bind _returnvalue (`Gauntlet_GameInstance.GetInputDevice` _gameinstance))
  (bind _returnvalue_2 (`Gauntlet_GameInstance.GetGameState` _gameinstance))
  (bind _returnvalue_3 (and (select `EGauntlet_GameState` _returnvalue_2 :`InMainMenu` true :`InPause` true) (select `EGauntlet_InputDevice` _returnvalue :`MouseKeyboard` true)))
  ; Show Cursor
  (set `self.bShowMouseCursor` _returnvalue_3)
  (`KismetSystemLibrary.PrintString` (`KismetStringLibrary.Concat_StrStr` "Show Mouse Cursor - " (`KismetStringLibrary.Conv_BoolToString` _returnvalue_3) " Game State - " (`|GetEnumeratorNameAsString` _returnvalue_2) " Input Device -" (`|GetEnumeratorNameAsString` _returnvalue)) true true (struct :`R` 1.0 :`G` 0.11988 :`A` 1.0) 2.0 "sdadsds"))

(fn `UserConstructionScript`)