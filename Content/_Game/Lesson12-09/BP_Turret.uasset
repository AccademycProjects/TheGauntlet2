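; BP_Turret is a turret that fires pooled projectiles automatically at a fixed interval.
; A looping timer started on BeginPlay calls Shoot every Delay seconds, which also prints a debug string.
; Shoot takes a BP_ProjectileBase from the pool, moves it to the Point component's location with the turret's rotation and its own root scale, then activates it, reusing projectiles rather than spawning them directly.
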(event `self.ReceiveBeginPlay`
  (`KismetSystemLibrary.K2_SetTimerDelegate` (delegate `Shoot`) (`self.Delay`) true))

(event `Shoot`
  (`KismetSystemLibrary.PrintString` "shoot" true true (struct :`G` 0.66 :`B` 1.0 :`A` 1.0) 2.0 "dsds")
  (bind _returnvalue (`/Game/_Game/Lesson12-09/BFL_ObjectPooling.GetProjectileFromPool` "/Game/_Game/Lesson12-09/BP_ProjectileBase.BP_ProjectileBase_C"))
  (bind _asbp_projectile_base (cast `/Game/_Game/Lesson12-09/BP_ProjectileBase` _returnvalue :!pure true))
  (`self.K2_SetActorTransform` _asbp_projectile_base (`KismetMathLibrary.MakeTransform` (`SceneComponent.K2_GetComponentLocation` (`self.Point`)) (`self.K2_GetActorRotation` self) (`SceneComponent.RelativeScale3D` (`/Game/_Game/Lesson12-09/BP_ProjectileBase.DefaultSceneRoot` _asbp_projectile_base))) false false)
  (`ObjectPoolInterface.BP_Activate` :`self` _returnvalue))

(fn `UserConstructionScript`)