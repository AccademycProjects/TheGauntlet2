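; BP_ProjectileBase is a pooled projectile base that is reused through activation and deactivation.
; Activate starts a lifetime timer, unhides the actor, tints its sphere green via a cached dynamic material and launches it along local X.
; Timer expiry or Hit, which clears the timer, returns it to the pool.
; If the material is valid, it then turns blue, waits briefly, hides and stops moving.
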(event `ObjectPoolInterface.BP_Activate`
  (params (ObjectPoolData :type "ObjectPoolActivationData Structure"))
  (bind _returnvalue (`KismetSystemLibrary.K2_SetTimerDelegate` (delegate `Deactivate`) (`self.LifeTime`)))
  (set `self.DeactivateLifeTimerHandle` _returnvalue)
  (`self.SetActorHiddenInGame` false)
  (`/Engine/EditorBlueprintResources/StandardMacros.IsValid` (`self.MID_Color`)
    (:`Is Valid`
      _)
    (:`Is Not Valid`
      (bind _returnvalue_2 (`PrimitiveComponent.CreateDynamicMaterialInstance` (`self.Sphere`) 0 "/Game/_Game/Lesson12-09/Material/M_Red.M_Red" "None"))
      (set `self.MID_Color` _returnvalue_2)))
  (`MaterialInstanceDynamic.SetVectorParameterValue` (`self.MID_Color`) "Color" (struct :`G` 1.0 :`A` 1.0))
  (`ProjectileMovementComponent.SetVelocityInLocalSpace` (`self.ProjectileMovement`) (`KismetMathLibrary.MakeVector` (`self.Speed`))))

(event `Deactivate`
  (`/Game/_Game/Lesson12-09/BFL_ObjectPooling.ReturnProjectileToPool` (`GameplayStatics.GetObjectClass` self) self :!label _label)
  (`/Engine/EditorBlueprintResources/StandardMacros.IsValid` (`self.MID_Color`)
    (:`Is Valid`
      (`MaterialInstanceDynamic.SetVectorParameterValue` (`self.MID_Color`) "Color" (struct :`B` 1.0 :`A` 1.0))
      (`KismetSystemLibrary.Delay` 0.2)
      (`self.SetActorHiddenInGame` true)
      (`ProjectileMovementComponent.SetVelocityInLocalSpace` (`self.ProjectileMovement`) (0.0 0.0 0.0)))))

(event `ObjectPoolInterface.BP_Deactivate`
  (params (DeactivationData :type "ObjectPoolDeactivationData Structure"))
  (goto _label))

(event `self.ReceiveHit`
  (params (MyComp :type "PrimitiveComponent Object Reference") (Other :type "Actor Object Reference") (OtherComp :type "PrimitiveComponent Object Reference") (bSelfMoved :type Boolean) (HitLocation :type "Vector Structure") (HitNormal :type "Vector Structure") (NormalImpulse :type "Vector Structure") (Hit :type "HitResult Structure (by ref)"))
  (`KismetSystemLibrary.K2_ClearAndInvalidateTimerHandle` (`self.DeactivateLifeTimerHandle`))
  (goto _label))

(fn `UserConstructionScript`)