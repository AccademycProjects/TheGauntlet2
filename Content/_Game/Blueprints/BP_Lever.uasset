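; BP_Lever is an interactable lever that shows an on or off position according to its Toggle component.
; On BeginPlay and on each toggle event, it sets the Pivot's relative rotation to AnimRotation when on, or that value multiplied by -1 when off, with no interpolation.
; An interaction event shows or hides the BPInteractionPrompt component.
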(event `self.OnInteractionPromptVisibilityChanged`
  (params (bVisible :type Boolean))
  (`SceneComponent.SetVisibility` (`self.BP_InteractionPrompt`) bVisible false))

(event `self.ReceiveBeginPlay`
  (bind _animrotation (`self.AnimRotation`))
  (bind _pivot (`self.Pivot`))
  (if (`ToggleComponent.IsOn` (`self.Toggle`))
    (`SceneComponent.K2_SetRelativeRotation` _pivot _animrotation false false :!label _label)
    (else
      (`SceneComponent.K2_SetRelativeRotation` _pivot (* _animrotation -1.0) false false :!label _label_2))))

(event `self.Toggle.OnToggleOnDelegate`
  (params (ToggleComponent :type "ToggleComponent Object Reference"))
  (goto _label))

(event `self.Toggle.OnToggleOffDelegate`
  (params (ToggleComponent :type "ToggleComponent Object Reference"))
  (goto _label_2))

(fn `UserConstructionScript`)